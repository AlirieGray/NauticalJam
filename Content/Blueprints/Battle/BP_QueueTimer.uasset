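; Battle queue timer that periodically drains each magical girl's ability queue.
; StartQueueTimer waits briefly, then starts a looping one-second timer on ExecuteCurrentAbilitiesInQueue.
; Each tick walks the MagicalGirlQueues map on the GameManagerSubsystem's AbilityQueueManager and dequeues one ability per key.
; The dequeued result is only printed as debug text; no ability is executed here.
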(event `StartQueueTimer`
  (`KismetSystemLibrary.PrintString` "Waiting")
  (`KismetSystemLibrary.Delay` 1.0)
  (`KismetSystemLibrary.PrintString` "starting timer!")
  (`KismetSystemLibrary.K2_SetTimer` null "ExecuteCurrentAbilitiesInQueue" 1.0 true))

(fn `ExecuteCurrentAbilitiesInQueue`
  (bind _returnvalue (`GameManagerSubsystem.GetAbilityQueueManager` (subsystem `GameManagerSubsystem`)))
  (bind _keypin (`|MapForEach` (`AbilityQueueManager.MagicalGirlQueues` _returnvalue))
    (:`then`
      (bind (_outsuccess _returnvalue_2) (`AbilityQueueManager.DequeueAbility` _returnvalue _keypin))
      (`KismetSystemLibrary.PrintString` (`KismetStringLibrary.BuildString_Name` (`KismetStringLibrary.Conv_BoolToString` _outsuccess) "DeQ ability for: " _keypin (`|GetEnumeratorNameAsString` (`.Name` (break `Ability` _returnvalue_2))))))))

(fn `UserConstructionScript`)