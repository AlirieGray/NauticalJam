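; BP_ManaManager tracks an integer mana pool, filling CurrentMana to MaxMana on BeginPlay.
; SetMana clamps the value between zero and MaxMana, and HasMana checks whether an amount is affordable.
; AddMana and RemoveMana clamp between zero and CurrentMana instead of MaxMana, so AddMana cannot raise the pool.
; The set, add and remove functions each return the updated value.
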(event `self.ReceiveBeginPlay`
  (set `self.CurrentMana` (`self.MaxMana`)))

(fn `AddMana`
  (params (Amount :type Integer))
  (returns (NewMana :type Integer))
  (bind _output_get (set `self.CurrentMana` (`KismetMathLibrary.Clamp` (+ Amount (`self.CurrentMana`)) 0 (`self.CurrentMana`))))
  (return _output_get))

(fn `HasMana`
  (params (Amount :type Integer))
  (returns (bHasAmount :type Boolean))
  (return (<= Amount (`self.CurrentMana`))))

(fn `RemoveMana`
  (params (Amount :type Integer))
  (returns (NewMana :type Integer))
  (bind _output_get (set `self.CurrentMana` (`KismetMathLibrary.Clamp` (- (`self.CurrentMana`) (`local.Amount`)) 0 (`self.CurrentMana`))))
  (return _output_get))

(fn `SetMana`
  (params (Amount :type Integer))
  (returns (NewMana :type Integer))
  (bind _output_get (set `self.CurrentMana` (`KismetMathLibrary.Clamp` Amount 0 (`self.MaxMana`))))
  (return _output_get))

(fn `UserConstructionScript`)