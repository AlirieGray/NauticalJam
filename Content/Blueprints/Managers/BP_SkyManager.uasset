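; Sky manager that switches the level's BP_GoodSky between day and night on demand.
; On BeginPlay it finds the sky, disables its automatic day/night cycle and activates it.
; Each switch event re-enables the cycle and actor tick, then starts a fast looping timer that polls the directional light's pitch.
; When pitch enters that state's narrow target window, it disables sky tick and clears the timer, freezing the time of day.
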(event `self.ReceiveBeginPlay`
  (bind _returnvalue (`GameplayStatics.GetActorOfClass` "/Game/GoodSky/Blueprint/BP_GoodSky.BP_GoodSky_C"))
  (set `self.MovingSky` _returnvalue)
  (set `/Game/GoodSky/Blueprint/BP_GoodSky.Enable Auto Day / Night Cycle In Game?` false (`self.MovingSky`))
  (`/Game/GoodSky/Blueprint/BP_GoodSky.Activate Sky` (`self.MovingSky`)))

(event `Switch to Night`
  (set `/Game/GoodSky/Blueprint/BP_GoodSky.Enable Auto Day / Night Cycle In Game?` true (`self.MovingSky`))
  (`self.SetActorTickEnabled` (`self.MovingSky`) true)
  (bind _returnvalue (`KismetSystemLibrary.K2_SetTimerDelegate` (delegate `Stop at Night`) 0.01 true))
  (set `self.TimeSwitchTimer` _returnvalue))

(event `Stop at Night`
  (bind (_returnvalue_roll _returnvalue_pitch) (`KismetMathLibrary.BreakRotator` (`self.K2_GetActorRotation` (`/Game/GoodSky/Blueprint/BP_GoodSky.└ Directional light actor ( For Custom Mode )` (`self.MovingSky`)))))
  (if (and (> _returnvalue_pitch 57.0) (< _returnvalue_pitch 59.0))
    (`self.SetActorTickEnabled` (`self.MovingSky`) false)
    (`KismetSystemLibrary.K2_ClearAndInvalidateTimerHandle` (`self.TimeSwitchTimer`))))

(event `Switch to Day`
  (set `/Game/GoodSky/Blueprint/BP_GoodSky.Enable Auto Day / Night Cycle In Game?` true (`self.MovingSky`))
  (`self.SetActorTickEnabled` (`self.MovingSky`) true)
  (bind _returnvalue (`KismetSystemLibrary.K2_SetTimerDelegate` (delegate `Stop at Day`) 0.01 true))
  (set `self.TimeSwitchTimer` _returnvalue))

(event `Stop at Day`
  (bind (_returnvalue_roll _returnvalue_pitch) (`KismetMathLibrary.BreakRotator` (`self.K2_GetActorRotation` (`/Game/GoodSky/Blueprint/BP_GoodSky.└ Directional light actor ( For Custom Mode )` (`self.MovingSky`)))))
  (if (and (> _returnvalue_pitch -59.0) (< _returnvalue_pitch -57.0))
    (`self.SetActorTickEnabled` (`self.MovingSky`) false)
    (`KismetSystemLibrary.K2_ClearAndInvalidateTimerHandle` (`self.TimeSwitchTimer`))))

(fn `UserConstructionScript`)