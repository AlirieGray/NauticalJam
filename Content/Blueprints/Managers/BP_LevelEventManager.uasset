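; Level event manager that switches the game between exploration and a boss battle.
; On BeginPlay it spawns the sky and music managers, then after a short delay puts the HUD and party player controller into exploration.
; Ending the day switches the sky to night and starts the battle, notifying the HUD, boss AI, player controller and camera.
; Cutting a battle short restores the camera and exploration UI; BattleWon is an empty stub.
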(event `self.ReceiveBeginPlay`
  (bind _returnvalue (`GameplayStatics.GetPlayerController` 0))
  (`|ExecutionSequence`
    (:`then_0`
      (bind _returnvalue_2 (`|SpawnActorFromClass` "/Game/Blueprints/Managers/BP_SkyManager.BP_SkyManager_C" (`KismetMathLibrary.MakeTransform` (0.0 0.0 0.0)) "Undefined" "MultiplyWithRoot" null null))
      (set `self.Sky Manager` _returnvalue_2)
      (bind _returnvalue_3 (`|SpawnActorFromClass` "/Game/Blueprints/Managers/BP_MusicManager.BP_MusicManager_C" (`KismetMathLibrary.MakeTransform` (0.0 0.0 0.0)) "Undefined" "MultiplyWithRoot" null null))
      (set `self.Music Manager` _returnvalue_3))
    (:`then_1`
      (`KismetSystemLibrary.Delay` 0.2)
      (message `/Game/Blueprints/Interfaces/BPI_HUD.CallExplorationUI` (`PlayerController.GetHUD` _returnvalue))
      (bind _asbp_player_controller_party_system (cast `/Game/Blueprints/PartySystem/BP_PlayerController_PartySystem` _returnvalue))
      (`/Game/Blueprints/PartySystem/BP_PlayerController_PartySystem.OnExplorationBegin` _asbp_player_controller_party_system))))

(event `Begin Battle`
  (message `/Game/Blueprints/Interfaces/BPI_HUD.CallBattleUI` (`PlayerController.GetHUD` (`GameplayStatics.GetPlayerController` 0)))
  (bind _returnvalue (`GameplayStatics.GetActorOfClass` "/Game/Blueprints/BossFight/BP_AIController_BossFight.BP_AIController_BossFight_C"))
  (`/Game/Blueprints/BossFight/BP_AIController_BossFight.StartFight` _returnvalue)
  (bind _asbp_player_controller_party_system (cast `/Game/Blueprints/PartySystem/BP_PlayerController_PartySystem` (`GameplayStatics.GetPlayerController` 0)))
  (`/Game/Blueprints/PartySystem/BP_PlayerController_PartySystem.OnBattleStart` _asbp_player_controller_party_system)
  (bind _returnvalue_2 (`GameplayStatics.GetActorOfClass` "/Game/Blueprints/PartySystem/BP_CameraController.BP_CameraController_C"))
  (`/Game/Blueprints/PartySystem/BP_CameraController.OnBattleStart` _returnvalue_2))

(event `BattleCutShort`
  (params (Phase :type Integer))
  (bind _returnvalue (`GameplayStatics.GetActorOfClass` "/Game/Blueprints/PartySystem/BP_CameraController.BP_CameraController_C"))
  (`/Game/Blueprints/PartySystem/BP_CameraController.OnBattleEnd` _returnvalue)
  (message `/Game/Blueprints/Interfaces/BPI_HUD.CallExplorationUI` (`PlayerController.GetHUD` (`GameplayStatics.GetPlayerController` 0))))

(event `BattleWon`)

(event `OnEndDay`
  (`/Game/Blueprints/Managers/BP_SkyManager.Switch to Night` (`self.Sky Manager`))
  (`KismetSystemLibrary.Delay` 1.0)
  (`self.Begin Battle`))

(fn `UserConstructionScript`)