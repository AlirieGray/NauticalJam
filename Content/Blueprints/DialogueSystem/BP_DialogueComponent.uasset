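; BP_DialogueComponent is a dialogue component that starts a behavior-tree-driven dialogue on its owning actor.
; RunDialogueTree runs BTAsset on the owner's AI controller, returning false when that controller is invalid.
; On success it reaches the first player's controller through GetPlayerMessage and adds its DialogueWidget to the viewport if not already shown.
; RunSingleDialogue accepts input text but is an empty stub.
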(event `self.ReceiveBeginPlay`)

(fn `RunDialogueTree`
  (returns (`Success?` :type Boolean))
  (bind _returnvalue (`AIBlueprintHelperLibrary.GetAIController` (`self.GetOwner`)))
  (`/Engine/EditorBlueprintResources/StandardMacros.IsValid` _returnvalue
    (:`Is Valid`
      (bind _returnvalue_2 (`AIController.RunBehaviorTree` _returnvalue (`self.BTAsset`)))
      (if _returnvalue_2
        (bind (_active_player _playercontroller) (message `/Game/Blueprints/Interfaces/BPI_Dialogue.GetPlayer` (`GameplayStatics.GetPlayerController` 0)))
        (bind _dialoguewidget (`/Game/Blueprints/PartySystem/BP_PlayerController_PartySystem.DialogueWidget` _playercontroller))
        (if (`Widget.IsInViewport` _dialoguewidget)
          (return _returnvalue_2)
          (else
            (`UserWidget.AddToViewport` _dialoguewidget 0)
            (return _returnvalue_2)))))
    (:`Is Not Valid`
      (return false))))

(fn `RunSingleDialogue`
  (params (InputText :type Text)))