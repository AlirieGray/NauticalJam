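; BP_Waves is an environment actor that bobs vertically, presumably to imitate wave motion.
; On BeginPlay it derives upper and lower Z limits from its starting height plus the MaxHeight and MinHeight offsets.
; A fast looping timer, used instead of Tick, moves the actor by a fixed Speed step, flipping the GoUp flag at each limit for a linear back-and-forth motion.
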(event `self.ReceiveBeginPlay`
  (bind (_returnvalue_x _returnvalue_y _returnvalue_z) (`KismetMathLibrary.BreakVector` (`self.K2_GetActorLocation`)))
  (bind (_returnvalue_x_2 _returnvalue_y_2 _returnvalue_z_2) (`KismetMathLibrary.BreakVector` (`self.K2_GetActorLocation`)))
  (set `self.MaxZ` (+ _returnvalue_z_2 (`self.MaxHeight`)))
  (set `self.MinZ` (+ _returnvalue_z (`self.MinHeight`)))
  (`KismetSystemLibrary.K2_SetTimerDelegate` (delegate `Bob`) 0.02 true))

(event `Bob`
  (bind (_returnvalue_x _returnvalue_y _returnvalue_z) (`KismetMathLibrary.BreakVector` (`self.K2_GetActorLocation`)))
  (bind (_returnvalue_x_2 _returnvalue_y_2 _returnvalue_z_2) (`KismetMathLibrary.BreakVector` (`self.K2_GetActorLocation`)))
  (bind (_returnvalue_x_3 _returnvalue_y_3 _returnvalue_z_3) (`KismetMathLibrary.BreakVector` (`self.K2_GetActorLocation`)))
  (bind (_returnvalue_x_4 _returnvalue_y_4 _returnvalue_z_4) (`KismetMathLibrary.BreakVector` (`self.K2_GetActorLocation`)))
  (if (`self.GoUp?`)
    (`self.K2_SetActorLocation` (`KismetMathLibrary.MakeVector` _returnvalue_x_4 _returnvalue_y_4 (+ _returnvalue_z_4 (`self.Speed`))))
    (if (>= _returnvalue_z (`self.MaxZ`))
      (set `self.GoUp?` false))
    (else
      (`self.K2_SetActorLocation` (`KismetMathLibrary.MakeVector` _returnvalue_x_3 _returnvalue_y_3 (- _returnvalue_z_3 (`self.Speed`))))
      (if (<= _returnvalue_z_2 (`self.MinZ`))
        (set `self.GoUp?` true)))))

(fn `UserConstructionScript`)