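; Boss battler for the boss fight that spawns and possesses its own AI controller, reporting health changes to the HUD.
; BossAttack maps an index to three DT_Abilities curse rows, executed through the Ability Manager with matching montages and Niagara effects.
; GetTargetS picks a random non-enemy, all non-enemies or self from Targets, which each attack overwrites.
; Defeat and interruption switch behavior trees and notify the level event manager.
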(event `self.ReceiveBeginPlay`
  (`KismetSystemLibrary.Delay` 5.0)
  (bind _outactors (`GameplayStatics.GetAllActorsOfClass` "/Script/NauticalJam.BattlerBase"))
  (set `self.Targets` _outactors)
  (bind _returnvalue (`|SpawnActorFromClass` "/Game/Blueprints/BossFight/BP_AIController_BossFight.BP_AIController_BossFight_C" (`KismetMathLibrary.MakeTransform` (0.0 0.0 0.0)) "Undefined" "MultiplyWithRoot" null null))
  (`Controller.Possess` _returnvalue self))

(event `self.OnDamageTaken`
  (params (Delta :type "Float (single-precision)"))
  ; On Damage Taken
  (`KismetSystemLibrary.PrintText` (`|FormatText` "Took {Damage} Damage! Health: {Current}/{Max}" Delta (`self.Health`) (`self.MaxHealth`)) true true (struct :`R` 1.0 :`A` 1.0))
  (message `/Game/Blueprints/Interfaces/BPI_HUD.UpdateBossHP` (`PlayerController.GetHUD` (`GameplayStatics.GetPlayerController` 0)) (`self.Health`) (`self.MaxHealth`)))

(event `self.OnHealed`
  (params (Delta :type "Float (single-precision)"))
  ; On Healed
  (`KismetSystemLibrary.PrintText` (`|FormatText` "Restored {Heal} Health! Health: {Current}/{Max}" Delta (`self.Health`) (`self.MaxHealth`)) true true (struct :`R` 1.0 :`A` 1.0))
  (message `/Game/Blueprints/Interfaces/BPI_HUD.UpdateBossHP` (`PlayerController.GetHUD` (`GameplayStatics.GetPlayerController` 0)) (`self.Health`) (`self.MaxHealth`)))

(event `/Game/Blueprints/Interfaces/BPI_BossFight.BossAttack`
  (params (AttackIndex :type Integer))
  (bind _target_s_ (`self.GetTarget(s)` true))
  (bind _target_s__2 (`self.GetTarget(s)` false false true))
  (bind _target_s__3 (`self.GetTarget(s)` false true))
  (switch `int` AttackIndex
    (:`1`
      (bind _returnvalue (`|GetDataTableRow` "/Game/Blueprints/MagicalGirl/Stats/DT_Abilities.DT_Abilities" "CurseBlast")
        (:`then`
          (`AbilityManager.ExecuteAbility` (`GameManagerSubsystem.GetAbilityManager` (subsystem `GameManagerSubsystem`)) self _returnvalue _target_s_)
          (set `self.Targets` _target_s_)
          (`self.LightAttack`))))
    (:`2`
      (bind _returnvalue_2 (`|GetDataTableRow` "/Game/Blueprints/MagicalGirl/Stats/DT_Abilities.DT_Abilities" "CurseShield")
        (:`then`
          (`AbilityManager.ExecuteAbility` (`GameManagerSubsystem.GetAbilityManager` (subsystem `GameManagerSubsystem`)) self _returnvalue_2 _target_s__2)
          (set `self.Targets` _target_s__2)
          (`self.Barrier`))))
    (:`3`
      (bind _returnvalue_3 (`|GetDataTableRow` "/Game/Blueprints/MagicalGirl/Stats/DT_Abilities.DT_Abilities" "CurseRain")
        (:`then`
          (`AbilityManager.ExecuteAbility` (`GameManagerSubsystem.GetAbilityManager` (subsystem `GameManagerSubsystem`)) self _returnvalue_3 _target_s__3)
          (set `self.Targets` _target_s__3)
          (`self.HeavyAttack`))))))

(event `BossDefeated`
  (`AIController.RunBehaviorTree` (`AIBlueprintHelperLibrary.GetAIController` self) "/Game/Blueprints/DialogueSystem/DialogueTrees/DT_Example4.DT_Example4")
  (bind _level_event_manager (message `/Game/Blueprints/Interfaces/BPI_GameInstance.GetLevelEventManger` (`GameplayStatics.GetGameInstance`)))
  (`/Game/Blueprints/Managers/BP_LevelEventManager.BattleWon` _level_event_manager))

(event `BattleInterrupted`
  (`AIController.RunBehaviorTree` (`AIBlueprintHelperLibrary.GetAIController` self) (select `int` (`self.Phase`) :`0` null :`1` "/Game/Blueprints/DialogueSystem/DialogueTrees/DT_Example4.DT_Example4" :`2` "/Game/Blueprints/DialogueSystem/DialogueTrees/DT_Example4.DT_Example4" :`3` "/Game/Blueprints/DialogueSystem/DialogueTrees/DT_Example4.DT_Example4" :!type "BehaviorTree Object Reference"))
  (bind _level_event_manager (message `/Game/Blueprints/Interfaces/BPI_GameInstance.GetLevelEventManger` (`GameplayStatics.GetGameInstance`)))
  (`/Game/Blueprints/Managers/BP_LevelEventManager.BattleCutShort` _level_event_manager (`self.Phase`)))

(event `LightAttack`
  (`|PlayMontage` (`self.SkeletalMesh`) "/Game/Characters/Mannequins/Anims/AM_ComboAttack.AM_ComboAttack"
    (:`then`
      (`NiagaraFunctionLibrary.SpawnSystemAtLocation` "/Game/Blueprints/BossFight/BossAttacks/N_CurseShield_Boss.N_CurseShield_Boss" (`self.K2_GetActorLocation` (`|GetArrayItem` (`self.Targets`)))))))

(event `Barrier`
  (`|PlayMontage` (`self.SkeletalMesh`) "/Game/Characters/Mannequins/Anims/AM_ChargedAttack.AM_ChargedAttack"
    (:`then`
      (`NiagaraFunctionLibrary.SpawnSystemAtLocation` "/Game/Blueprints/BossFight/BossAttacks/N_EnergyShield_Boss.N_EnergyShield_Boss" (`self.K2_GetActorLocation` (`|GetArrayItem` (`self.Targets`)))))))

(event `HeavyAttack`
  (`|PlayMontage` (`self.SkeletalMesh`) "/Game/Characters/Mannequins/Anims/AM_ComboAttack.AM_ComboAttack"
    (:`then`
      (for _array_element (`self.Targets`)
        (`NiagaraFunctionLibrary.SpawnSystemAtLocation` "/Game/Blueprints/BossFight/BossAttacks/N_MagicalMeteorShower_Boss.N_MagicalMeteorShower_Boss" (`self.K2_GetActorLocation` _array_element))))))

(fn `GetTarget(s)`
  (params (`SingleTarget?` :type Boolean) (`MultiTarget?` :type Boolean) (`SelfTarget?` :type Boolean))
  (returns (`Target(s)` :type "Array of BattlerBase Object Reference"))
  (locals (L_Targets :type "Array of BattlerBase Object Reference"))
  (if `SingleTarget?`
    (for _array_element (`self.Targets`)
      (if (not (`BattlerBase.Enemy` _array_element))
        (`KismetArrayLibrary.Array_AddUnique` (`local.L_Targets`) _array_element)))
    (return (`|MakeArray` (`KismetArrayLibrary.Array_Random` (`local.L_Targets`))))
    (elif `MultiTarget?`
      (for _array_element_2 (`self.Targets`)
        (if (not (`BattlerBase.Enemy` _array_element_2))
          (`KismetArrayLibrary.Array_AddUnique` (`local.L_Targets`) _array_element_2)))
      (return (`local.L_Targets`))
      (elif `SelfTarget?`
        (return (`|MakeArray` self))
        (else
          (return (`|MakeArray` null :!type "BattlerBase Object Reference")))))))

(fn `UpdateBossHP_OLD`
  (message `/Game/Blueprints/Interfaces/BPI_HUD.UpdateBossHP` (`PlayerController.GetHUD` (`GameplayStatics.GetPlayerController` 0)) 0.0 0.0))

(fn `UserConstructionScript`)