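; Action queue Blueprint that keeps a separate list of pending abilities for each magical girl, looked up by name.
; EnqueueAbility appends while the list length is at or below a cap, otherwise printing that it is full.
; BeginQueueLoop sets a looping timer on DequeueAbilityAndExecute, which takes a name parameter and only removes the first entry, without executing it.
; StopQueueLoop is an empty stub.
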(event `BeginQueueLoop`
  (`KismetSystemLibrary.K2_SetTimer` null "DequeueAbilityAndExecute" 2.0 true))

(event `StopQueueLoop`)

(fn `DequeueAbilityAndExecute`
  (params (MagicalGirlName :type Name))
  (`KismetArrayLibrary.Array_Remove` (`.Abilities_6_88ACE99E4A47F0154BCD11B21353F14A` (break `/Game/Blueprints/MagicalGirl/ActionQueueSystem/S_Queue` (`BlueprintMapLibrary.Map_Find` (`self.Queues`) (`local.MagicalGirlName`))))))

(fn `EnqueueAbility`
  (params (MagicalGirlName :type Name) (Ability :type "/Game/Blueprints/MagicalGirl/Abilities/S_Ability_MagicalGirl Structure"))
  (if (<= (`KismetArrayLibrary.Array_Length` (`.Abilities_6_88ACE99E4A47F0154BCD11B21353F14A` (break `/Game/Blueprints/MagicalGirl/ActionQueueSystem/S_Queue` (`BlueprintMapLibrary.Map_Find` (`self.Queues`) (`local.MagicalGirlName`))))) (`self.MaxAbilitiesInQ`))
    (`KismetArrayLibrary.Array_Add` (`.Abilities_6_88ACE99E4A47F0154BCD11B21353F14A` (break `/Game/Blueprints/MagicalGirl/ActionQueueSystem/S_Queue` (`BlueprintMapLibrary.Map_Find` (`self.Queues`) (`local.MagicalGirlName`)))) (`local.Ability`))
    (else
      (`KismetSystemLibrary.PrintString` "Q full"))))

(fn `UserConstructionScript`)