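; Magical girl character that moves by Enhanced Input and returns to its cached AI controller when unpossessed.
; Damage and healing send clamped health percentages to the HUD interface without storing CurrentHealth.
; Abilities spend mana when affordable and update the HUD, but only print their name.
; A looping timer targets "RegenMana", while the Clairvoyance-scaled regen function is named ManaRegn and does not update the HUD.
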(event `self.ReceiveBeginPlay`
  (bind _returnvalue (`GameplayStatics.GetPlayerController` 0))
  (bind (_stats_maxhealth _stats_maxmana) (break `/Game/Blueprints/MagicalGirl/S_MagicalGirlStats` (`self.Stats`)))
  (set `self.CurrentHealth` _stats_maxhealth)
  (set `self.CurrentMana` _stats_maxmana)
  (bind _asbp_magical_girl_aicontroller (cast `/Game/Blueprints/PartySystem/BP_MagicalGirlAIController` (`AIBlueprintHelperLibrary.GetAIController` self)))
  (set `self.MagicalGirlAIController` _asbp_magical_girl_aicontroller)
  (`EnhancedInputSubsystemInterface.AddMappingContext` (pcsubsystem `EnhancedInputLocalPlayerSubsystem` _returnvalue) null 0 (struct))
  (bind _asbpi_hud (cast `/Game/Blueprints/Interfaces/BPI_HUD` (`PlayerController.GetHUD` _returnvalue)))
  (set `self.HUD` _asbpi_hud))

(event `self.ReceiveUnpossessed`
  (params (OldController :type "Controller Object Reference"))
  (`/Engine/EditorBlueprintResources/StandardMacros.IsValid` (`self.MagicalGirlAIController`)
    (:`Is Valid`
      (`Controller.Possess` (`self.MagicalGirlAIController`) self))))

(event `EnhancedInput|/Game/Input/Actions/IA_Move`
  (params (ActionValue :type "Vector2D Structure") (ElapsedSeconds :type "Float (double-precision)") (TriggeredSeconds :type "Float (double-precision)") (InputAction :type "InputAction Object Reference" :default "/Game/Input/Actions/IA_Move.IA_Move"))
  (bind (_x _y) (`KismetMathLibrary.BreakVector2D` ActionValue))
  (:`Triggered`
    (`self.AddMovementInput` (`KismetMathLibrary.MakeVector` _y _x))))

(event `self.ReceivePossessed`
  (params (NewController :type "Controller Object Reference")))

(event `self.ReceiveAnyDamage`
  (params (Damage :type "Float (single-precision)") (DamageType :type "DamageType Object Reference") (InstigatedBy :type "Controller Object Reference") (DamageCauser :type "Actor Object Reference"))
  (`self.OnTakeDamage` Damage))

(event `StartManaRegenTimer`
  (bind _returnvalue (`KismetSystemLibrary.K2_SetTimer` null "RegenMana" 1.0 true))
  (set `self.ManaRegenTimer` _returnvalue))

(event `StopManaRegenTimer`
  (`KismetSystemLibrary.K2_ClearAndInvalidateTimerHandle` (`self.ManaRegenTimer`)))

(fn `ExecuteAbility`
  (params (Ability :type "/Game/Blueprints/MagicalGirl/Abilities/S_Ability_MagicalGirl Structure"))
  (returns (`Success?` :type Boolean))
  (locals (L_ManaCost :type "Float (double-precision)"))
  (bind (_name _manacost) (break `/Game/Blueprints/MagicalGirl/Abilities/S_Ability_MagicalGirl` Ability))
  (set `local.L_ManaCost` _manacost)
  (if (>= (- (`self.CurrentMana`) _manacost) 0.0)
    (`self.OnSpendMana` (`local.L_ManaCost`))
    (`KismetSystemLibrary.PrintString` "ExecutingAbility:")
    (`KismetSystemLibrary.PrintString` (`KismetStringLibrary.Conv_NameToString` (`.Name_2_092C3D014B1D7B342086F0BC625229A0` (break `/Game/Blueprints/MagicalGirl/Abilities/S_Ability_MagicalGirl` (`local.Ability`)))))
    (return true)
    (else
      (return false))))

(fn `GetCurrentMana`
  (returns (Mana :type "Float (double-precision)"))
  (return (`self.CurrentMana`)))

(fn `GetManaRegenRateFromClairvoyance`
  (returns (ManaRegenPerSecond :type "Float (double-precision)"))
  (bind (_stats_maxhealth _stats_maxmana _stats_sleuth _stats_clairvoyance) (break `/Game/Blueprints/MagicalGirl/S_MagicalGirlStats` (`self.Stats`)))
  (return (/ _stats_clairvoyance 25.0)))

(fn `GetPlayer`
  (returns (`Active Player` :type "/Game/Blueprints/MagicalGirl/BP_MagicalGirlCharacter Object Reference") (PlayerController :type "/Game/Blueprints/PartySystem/BP_PlayerController_PartySystem Object Reference"))
  (return self null))

(fn `Heal`
  (params (HealAmt :type "Float (double-precision)"))
  (bind _stats_maxhealth (break `/Game/Blueprints/MagicalGirl/S_MagicalGirlStats` (`self.Stats`)))
  (`/Game/Blueprints/Interfaces/BPI_HUD.UpdatePlayerHP` (`self.HUD`) (`self.Name`) (/ (`KismetMathLibrary.FClamp` (+ (`self.CurrentHealth`) (`local.HealAmt`)) 0.0 _stats_maxhealth) _stats_maxhealth)))

(fn `ManaRegn`
  (bind (_stats_maxhealth _stats_maxmana) (break `/Game/Blueprints/MagicalGirl/S_MagicalGirlStats` (`self.Stats`)))
  (bind _manaregenpersecond (`self.GetManaRegenRateFromClairvoyance`))
  (set `self.CurrentMana` (`KismetMathLibrary.FClamp` (+ (`self.CurrentMana`) _manaregenpersecond) 0.0 _stats_maxmana)))

(fn `OnSpendMana`
  (params (ManaAmt :type "Float (double-precision)"))
  (bind (_stats_maxhealth _stats_maxmana) (break `/Game/Blueprints/MagicalGirl/S_MagicalGirlStats` (`self.Stats`)))
  (bind _output_get (set `self.CurrentMana` (`KismetMathLibrary.FClamp` (- (`self.CurrentMana`) ManaAmt) 0.0 _stats_maxmana)))
  (`/Game/Blueprints/Interfaces/BPI_HUD.UpdatePlayerMana` (`self.HUD`) (`self.Name`) (/ _output_get _stats_maxmana)))

(fn `OnTakeDamage`
  (params (DamageAmt :type "Float (double-precision)"))
  (bind _stats_maxhealth (break `/Game/Blueprints/MagicalGirl/S_MagicalGirlStats` (`self.Stats`)))
  (`/Game/Blueprints/Interfaces/BPI_HUD.UpdatePlayerHP` (`self.HUD`) (`self.Name`) (/ (`KismetMathLibrary.FClamp` (- (`self.CurrentHealth`) (`local.DamageAmt`)) 0.0 _stats_maxhealth) _stats_maxhealth)))

(fn `SetMovementEnabled`
  (params (EnableMovement :type Boolean))
  (bind _output_get (set `self.Enable Movement` EnableMovement))
  (if _output_get
    (`CharacterMovementComponent.SetMovementMode` (`self.CharacterMovement`) "MOVE_Walking" 0)
    (else
      (`CharacterMovementComponent.DisableMovement` (`self.CharacterMovement`)))))

(fn `UserConstructionScript`)