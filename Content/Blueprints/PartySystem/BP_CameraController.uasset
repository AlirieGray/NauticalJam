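; Party system camera controller that glides its camera component after a follow target.
; SetFollowTarget stores the target actor, and a looping timer started at BeginPlay calls GlideToTarget every hundredth of a second instead of using Tick.
; Each call interpolates from the camera's current location toward the target with a fixed delta time, then adds ViewOffset to the result.
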(event `self.ReceiveBeginPlay`
  (`KismetSystemLibrary.K2_SetTimer` null "GlideToTarget" 0.01 true))

(fn `GlideToTarget`
  (`/Engine/EditorBlueprintResources/StandardMacros.IsValid` (`self.FollowTarget`)
    (:`Is Valid`
      (`SceneComponent.K2_SetWorldLocation` (`self.CameraComponent`) (+ (`KismetMathLibrary.VInterpTo` (`SceneComponent.K2_GetComponentLocation` (`self.CameraComponent`)) (`self.K2_GetActorLocation` (`self.FollowTarget`)) 1.0 0.5) (`self.ViewOffset`)) false false))))

(fn `SetFollowTarget`
  (params (NewFollowTarget :type "Actor Object Reference"))
  (set `self.FollowTarget` NewFollowTarget))

(fn `UserConstructionScript`)