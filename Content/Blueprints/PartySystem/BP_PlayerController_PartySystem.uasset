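; Player controller for the party system that lets the player cycle control between spawned party pawns.
; On BeginPlay it subscribes to the manager pawn's spawn event, then stores the pawns and possesses the one at the current index.
; The switch-character input advances that index with wraparound and possesses the next pawn.
; After each possession, the view targets BP_CameraController, which is set to follow the active pawn.
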(event `self.ReceiveBeginPlay`
  (bind _asbp_manager_pawn (cast `/Game/Blueprints/PartySystem/BP_ManagerPawn` (`self.K2_GetPawn`)))
  (add `/Game/Blueprints/PartySystem/BP_ManagerPawn.PawnsSpawned` _asbp_manager_pawn (delegate `AssumeControl`)))

(event `AssumeControl`
  (params (Pawns :type "Array of Pawn Object Reference (by ref)"))
  (bind _output_get (set `self.Pawns` Pawns))
  (bind _output (`|GetArrayItem` _output_get (`self.CurrentMGIndex`)))
  (`self.Possess` _output)
  (bind _returnvalue (`GameplayStatics.GetActorOfClass` "/Game/Blueprints/PartySystem/BP_CameraController.BP_CameraController_C"))
  (`self.SetViewTargetWithBlend` _returnvalue)
  (`/Game/Blueprints/PartySystem/BP_CameraController.SetFollowTarget` _returnvalue _output))

(event `EnhancedInput|/Game/Input/Actions/IA_SwitchCharacter`
  (params (ActionValue :type Boolean) (ElapsedSeconds :type "Float (double-precision)") (TriggeredSeconds :type "Float (double-precision)") (InputAction :type "InputAction Object Reference" :default "/Game/Input/Actions/IA_SwitchCharacter.IA_SwitchCharacter"))
  (:`Triggered`
    (`self.OnSwitchControlledCharacter`)))

(fn `OnSwitchControlledCharacter`
  (locals (L_CurrentIndexPlusOne :type Integer))
  (bind _output (`|GetArrayItem` (`self.Pawns`) (`self.CurrentMGIndex`)))
  (bind _returnvalue (+ (`self.CurrentMGIndex`) 1))
  (`KismetSystemLibrary.PrintString` "SWITCHING")
  (set `local.L_CurrentIndexPlusOne` _returnvalue)
  (if (>= _returnvalue (`KismetArrayLibrary.Array_Length` (`self.Pawns`)))
    (set `self.CurrentMGIndex` 0)
    (else
      (set `self.CurrentMGIndex` (`local.L_CurrentIndexPlusOne`))))
  (`self.Possess` _output)
  (bind _returnvalue_2 (`GameplayStatics.GetActorOfClass` "/Game/Blueprints/PartySystem/BP_CameraController.BP_CameraController_C"))
  (`self.SetViewTargetWithBlend` _returnvalue_2)
  (`/Game/Blueprints/PartySystem/BP_CameraController.SetFollowTarget` _returnvalue_2 _output))

(fn `UserConstructionScript`)