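; Party-system magical girl character that hands itself back to AI control whenever another controller releases it.
; BeginPlay caches its AI controller, and Unpossessed has that cached controller repossess the pawn if still valid.
; The construction script writes the character's Name into a placeholder text component.
; Possession and mouse-look input only print debug strings, and the input mapping context setup is left unconnected.
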(event `self.ReceiveBeginPlay`
  (bind _asbp_magical_girl_aicontroller (cast `/Game/Blueprints/PartySystem/BP_MagicalGirlAIController` (`AIBlueprintHelperLibrary.GetAIController` self)))
  (set `self.MagicalGirlAIController` _asbp_magical_girl_aicontroller))

(event `self.ReceiveUnpossessed`
  (params (OldController :type "Controller Object Reference"))
  (`/Engine/EditorBlueprintResources/StandardMacros.IsValid` (`self.MagicalGirlAIController`)
    (:`Is Valid`
      (`Controller.Possess` (`self.MagicalGirlAIController`) self))))

(event `self.ReceivePossessed`
  (params (NewController :type "Controller Object Reference"))
  (`KismetSystemLibrary.PrintString` "POSESSED: ")
  (`KismetSystemLibrary.PrintString` (`KismetStringLibrary.Conv_NameToString` (`self.Name`))))

(event `EnhancedInput|/Game/Input/Actions/IA_MouseLook`
  (params (ActionValue :type "Vector2D Structure") (ElapsedSeconds :type "Float (double-precision)") (TriggeredSeconds :type "Float (double-precision)") (InputAction :type "InputAction Object Reference" :default "/Game/Input/Actions/IA_MouseLook.IA_MouseLook"))
  (:`Triggered`
    (`KismetSystemLibrary.PrintString` "dont look!")))

(fn `UserConstructionScript`
  (`TextRenderComponent.K2_SetText` (`self.CharacterName_Placeholder`) (`KismetTextLibrary.Conv_NameToText` (`self.Name`))))