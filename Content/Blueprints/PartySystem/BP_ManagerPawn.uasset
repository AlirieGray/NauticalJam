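; BP_ManagerPawn is the party system's manager pawn, spawning the group of magical girl characters at game start.
; After a short BeginPlay delay, SpawnPawns creates one BP_MagicalGirlCharacter per MagicalGirlPawnInfo entry, placed at the manager's location plus that entry's offset.
; Spawns adjust for collisions but always succeed, and the resulting array is broadcast through PawnsSpawned.
; Each entry's Name is read but unused.
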(event `self.ReceiveBeginPlay`
  (`KismetSystemLibrary.Delay` 0.2)
  (bind _pawnstopossess (`self.SpawnPawns` (`self.MagicalGirlPawnInfo`)))
  (`self.PawnsSpawned` _pawnstopossess))

(fn `SpawnPawns`
  (params (PawnInfo :type "Array of /Game/Blueprints/PartySystem/S_MagicalGirlPawnInfo Structure"))
  (returns (PawnsToPossess :type "Array of Pawn Object Reference"))
  (locals (L_Pawns :type "Array of Pawn Object Reference") (L_MGName :type Name) (L_MGSpawnOffset :type "Vector Structure"))
  (for _index (range (+ (`KismetArrayLibrary.Array_LastIndex` PawnInfo) 1))
    (bind (_output_name _output_spawnoffset) (break `/Game/Blueprints/PartySystem/S_MagicalGirlPawnInfo` (`|GetArrayItem` PawnInfo _index)))
    (set `local.L_MGName` _output_name)
    (set `local.L_MGSpawnOffset` _output_spawnoffset)
    (bind _returnvalue (`|SpawnActorFromClass` "/Game/Blueprints/MagicalGirl/BP_MagicalGirlCharacter.BP_MagicalGirlCharacter_C" (`KismetMathLibrary.MakeTransform` (+ (`self.K2_GetActorLocation`) (`local.L_MGSpawnOffset`))) "AdjustIfPossibleButAlwaysSpawn" "MultiplyWithRoot" null null))
    (`KismetArrayLibrary.Array_Add` (`local.L_Pawns`) _returnvalue))
  (return (`local.L_Pawns`)))

(fn `UserConstructionScript`)